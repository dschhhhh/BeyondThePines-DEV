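; Ground pathway tile that scatters random trees, rocks and branches over itself at BeginPlay.
; A zero-second Delay first lets the generator's transform changes land, then three sequential while loops spawn props up to randomly rolled counts.
; Each prop gets a random position within SpawnVolume's extents around the actor, plus random rotation and scale.
; Loops spawn before comparing counts, so a zero branch roll still yields one branch.
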(event EventBeginPlay)

(event Collision|EventActorBeginOverlap
  (params (OtherActor :type Actor%20Object%20Reference)))

(event EventTick
  (params (DeltaSeconds :type Float%20%28single-precision%29)))

(event EventBeginPlay
  (bind _returnvalue (Transformation|GetActorLocation))
  (bind _returnvalue_2 (Math|Random|RandomIntegerinRange 0 360))
  (bind _returnvalue_3 (Math|Random|RandomFloatinRange 0.65 1.0))
  (bind _spawnvolume (Variables|Default|GetSpawnVolume))
  (bind _returnvalue_4 (Components|Box|GetScaledBoxExtent _spawnvolume))
  (bind _returnvalue_5 (Math|Conversions|ToFloat(Integer) _returnvalue_2))
  (bind (_x _y) (Math|Vector|BreakVector _returnvalue_4))
  (bind _returnvalue_6 (Math|Rotator|MakeRotator 0.0 0.0 _returnvalue_5))
  (bind _returnvalue_7 (* _y -1.0))
  (bind _returnvalue_8 (* _x -1.0))
  (bind _returnvalue_9 (Math|Random|RandomFloatinRange _returnvalue_8 _x))
  (bind _returnvalue_10 (Math|Random|RandomFloatinRange _returnvalue_7 _y))
  (bind _returnvalue_11 (Math|Vector|MakeVector _returnvalue_9 _returnvalue_10 2e+01))
  (bind _returnvalue_12 (+ _returnvalue_11 _returnvalue))
  (Utilities|FlowControl|Delay 0.0) ; Delay to let transform changes happen in generator before spawning
  ;[1 1 1] Tree generation
  (Variables|Default|SetMaxTrees_onTile (Math|Random|RandomIntegerinRange 1 3))
  (while (Variables|Default|GetMaxTreesNotReached) :!label _label
    (Game|SpawnActorfromClass "/Game/ProjectBase/Blueprint/Tree_3m_Blueprint.Tree_3m_Blueprint_C" (Math|Transform|MakeTransform _returnvalue_12 _returnvalue_6 (Math|Conversions|ToVector(Float) (Math|Random|RandomFloatinRange 0.25 0.75))) "AdjustIfPossibleButAlwaysSpawn" 0 0 0)
    (bind _output_get (Variables|Default|SetCurrentMaxTrees (+ (Variables|Default|GetCurrentMaxTrees) 1)))
    (Math|Integer|CompareInt _output_get (Variables|Default|GetMaxTrees_onTile)
      (:>
        _)
      (:==
        _)
      (:<
        (goto _label)))
    (Variables|Default|SetMaxTreesNotReached false)
    (goto _label))
  ;[1 1 1] Rock generation
  (Variables|Default|SetMaxRocks_onTile (Math|Random|RandomIntegerinRange 1 5))
  (while (Variables|Default|GetMaxRocks_notReached) :!label _label_2
    (Game|SpawnActorfromClass "/Game/ProjectBase/Blueprints/Rock_2m_Blueprint.Rock_2m_Blueprint_C" (Math|Transform|MakeTransform _returnvalue_12 (Math|Rotator|MakeRotator _returnvalue_5 _returnvalue_5 _returnvalue_5) (Math|Conversions|ToVector(Float) _returnvalue_3)) "AdjustIfPossibleButAlwaysSpawn" 0 0)
    (bind _output_get_2 (Variables|Default|SetCurrentMaxRocks (+ (Variables|Default|GetCurrentMaxRocks) 1)))
    (Math|Integer|CompareInt _output_get_2 (Variables|Default|GetMaxRocks_onTile)
      (:>
        _)
      (:==
        _)
      (:<
        (goto _label_2)))
    (Variables|Default|SetMaxRocks_notReached false)
    (goto _label_2))
  ;[1 1 1] Branch generation
  (Variables|Default|SetMaxBranches_onTile (Math|Random|RandomIntegerinRange 0 2))
  (while (Variables|Default|GetMaxBranches_notReached) :!label _label_3
    (Game|SpawnActorfromClass "/Game/ProjectBase/Blueprint/Branch_Blueprint.Branch_Blueprint_C" (Math|Transform|MakeTransform _returnvalue_12 _returnvalue_6 (Math|Conversions|ToVector(Float) _returnvalue_3)) "AdjustIfPossibleButAlwaysSpawn" 0 0)
    (bind _output_get_3 (Variables|Default|SetCurrentMaxBranches (+ (Variables|Default|GetCurrentMaxBranches) 1)))
    (Math|Integer|CompareInt _output_get_3 (Variables|Default|GetMaxBranches_onTile)
      (:>
        _)
      (:==
        _)
      (:<
        (goto _label_3)))
    (Variables|Default|SetMaxBranches_notReached false)
    (goto _label_3)))

(fn ConstructionScript)

(fn GetAttachTransform
  (return ""))