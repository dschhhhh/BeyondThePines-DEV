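; Spawner that procedurally builds a path of ground pieces from a start piece at BeginPlay, then places a GeoCache.
; A wired-back execution loop spawns random ground pieces until the count reaches WorldSize.
; Each piece is offset from the previous one by their combined bounds along +X, +Y or -Y.
; The GeoCache lands on a random piece from the later part of the path; overlap checking and rotation are unfinished and unconnected.
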(event EventBeginPlay)

(event EventBeginPlay
  (bind _existingpieces (Variables|Default|GetExistingPieces))
  (bind _returnvalue (Game|SpawnActorfromClass (Utilities|Select :Index 0 :Option%200 "/Game/ProjectBase/Blueprint/Ground_PlayerStart.Ground_PlayerStart_C" :Option%201 "/Game/ProjectBase/Blueprint/Ground_PlayerStart.Ground_PlayerStart_C") (Transformation|GetActorTransform) "AdjustIfPossibleButAlwaysSpawn" 0 0))
  (bind _output_get (Variables|Default|SetLastSpawned _returnvalue))
  (Variables|Default|SetNewlySpawned _output_get)
  (Utilities|FlowControl|Delay 0.1)
  ;[1 1 1] Comparing against worldsize
  (bind _output_get_2 (Variables|Default|SetCurrent%20pieces (+ (Variables|Default|GetCurrent%20pieces) 1) :!label _label))
  (Math|Integer|CompareInt _output_get_2 (Variables|Default|GetWorld%20Size)
    (:>
      _)
    (:==
      _)
    (:<
      (bind _returnvalue_2 (Game|SpawnActorfromClass (Utilities|Select :Index (Math|Random|RandomIntegerinRange (Variables|Default|GetFirst%20Index) (Utilities|Array|LastIndex (Variables|Default|GetActors))) :Option%200 "/Game/ProjectBase/Blueprint/Ground_10.Ground_10_C" :Option%201 "/Game/ProjectBase/Blueprint/Ground_20.Ground_20_C" :Option%202 "/Game/ProjectBase/Blueprint/Ground_Pathway.Ground_Pathway_C") (Transformation|GetActorTransform (Variables|Default|GetLastSpawned)) "AdjustIfPossibleButAlwaysSpawn" 0 0))
      (Transformation|AddActorWorldOffset _returnvalue_2 (Utilities|Select :Index (Math|Random|RandomInteger 2) :Option%200 (Math|Vector|MakeVector (.X (Math|Vector|BreakVector (+ (.BoxExtent (Collision|GetActorBounds _returnvalue_2 false)) (.BoxExtent (Collision|GetActorBounds (Variables|Default|GetNewlySpawned) false))))) 0.0 0.0) :Option%201 (Utilities|Select :Index (Math|Random|RandomInteger 2) :Option%200 (Math|Vector|MakeVector 0.0 (.Y (Math|Vector|BreakVector (+ (.BoxExtent (Collision|GetActorBounds _returnvalue_2 false)) (.BoxExtent (Collision|GetActorBounds (Variables|Default|GetNewlySpawned) false))))) 0.0) :Option%201 (Math|Vector|MakeVector 0.0 (* (.Y (Math|Vector|BreakVector (+ (.BoxExtent (Collision|GetActorBounds _returnvalue_2 false)) (.BoxExtent (Collision|GetActorBounds (Variables|Default|GetNewlySpawned) false))))) -1.0) 0.0))))
      (bind _output_get_3 (Variables|Default|SetNewlySpawned _returnvalue_2))
      (bind _output_get_4 (Variables|Default|SetLastSpawned _output_get_3))
      (Utilities|Array|Add (Variables|Default|GetExistingPieces) _output_get_4)
      (goto _label)))
  (Game|SpawnActorfromClass "/Game/ProjectBase/Blueprint/GeoCache_Blueprint.GeoCache_Blueprint_C" (Transformation|GetActorTransform (Utilities|Array|Get(acopy) _existingpieces (Math|Random|RandomIntegerinRange (/ (Variables|Default|GetWorld%20Size) 2) (Utilities|Array|LastIndex _existingpieces)))) "Undefined" 0 0)
  (Variables|Default|SetWorldSize_notReached false))

(fn ConstructionScript)