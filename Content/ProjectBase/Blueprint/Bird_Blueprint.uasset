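; Bird actor that flies between random perch points on nearby trees.
; From BeginPlay it finds Tree_3m_Blueprint actors overlapping its SearchArea, then picks a random tree and one of its BirdTargets.
; A timeline lerps the current location and rotation toward that perch, facing the direction of travel.
; The timeline's Update also starts a random Delay that loops back to choose the next perch.
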(event EventBeginPlay)

(event Collision|EventActorBeginOverlap
  (params (OtherActor :type Actor%20Object%20Reference)))

(event EventBeginPlay
  (bind _returnvalue (Transformation|GetActorLocation))
  (bind _searcharea (Variables|Default|GetSearchArea))
  (bind _overlappingactors (Collision|GetOverlappingActors _searcharea "/Game/ProjectBase/Blueprint/Tree_3m_Blueprint.Tree_3m_Blueprint_C" :!class /Script/Engine.PrimitiveComponent))
  (Utilities|FlowControl|Delay 1.0 :!label _label)
  (bind _output_get (Variables|Default|SetFoundTrees _overlappingactors))
  (Utilities|FlowControl|Delay 2.0)
  (bind _astree_3m_blueprint (Utilities|Casting|CastToTree_3m_Blueprint (Utilities|Array|Get(acopy) _output_get (Math|Random|RandomIntegerinRange 0 (Utilities|Array|LastIndex _overlappingactors)))))
  (Variables|Default|SetTreeLocation (Transformation|GetWorldLocation (Utilities|Array|Get(acopy) (Variables|/Game/ProjectBase/Blueprint/Tree_3m_Blueprint.Tree_3m_Blueprint_C|GetBirdTargets _astree_3m_blueprint) (Math|Random|RandomIntegerinRange 0 (Utilities|Array|LastIndex (Variables|/Game/ProjectBase/Blueprint/Tree_3m_Blueprint.Tree_3m_Blueprint_C|GetBirdTargets _astree_3m_blueprint))))))
  (bind _speed (Timeline|Timeline_0 PlayFromStart)
    (:Update
      (Transformation|SetActorLocationAndRotation (Math|Vector|Lerp(Vector) _returnvalue (Variables|Default|GetTreeLocation) _speed) (Math|Rotator|Lerp(Rotator) (Transformation|GetActorRotation) (Math|Conversions|RotationFromXVector (Math|Vector|GetUnitDirection(Vector) _returnvalue (Variables|Default|GetTreeLocation))) _speed))
      (Utilities|FlowControl|Delay (Math|Random|RandomFloatinRange 5.0 25.0))
      (goto _label))))

(fn ConstructionScript)