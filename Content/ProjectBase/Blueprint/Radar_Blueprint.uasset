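; Radar HUD Blueprint that plots GeoCache actors within a set radius around the player, redrawn on BeginPlay and Tick.
; DrawRadar maps each actor's offset from the player into radar space, then rotates it by control yaw.
; Location, player and background materials go to DrawSmartTexture, which scales coordinates from a 1080p reference.
; Its DrawMaterialSimple call is disconnected, so nothing renders, and GetTempOffset ignores the stored start position.
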(event EventBeginPlay
  (CallFunction|DrawRadar "(X=512.000000,Y=512.000000)" 9e+02 5e+02))

(event Collision|EventActorBeginOverlap
  (params (OtherActor :type Actor%20Object%20Reference)))

(event EventTick
  (params (DeltaSeconds :type Float%20%28single-precision%29))
  (CallFunction|DrawRadar "(X=512.000000,Y=512.000000)" 9e+02 5e+02))

(fn ConstructionScript
  (bind _returnvalue (Rendering|Material|CreateDynamicMaterialInstance 0 "None" :!class /Script/Engine.KismetMaterialLibrary))
  (Variables|Default|SetRadarBG _returnvalue)
  (bind _returnvalue_2 (Rendering|Material|CreateDynamicMaterialInstance "/Game/ProjectBase/Materials/M_Cursor_Feet.M_Cursor_Feet" "None" :!class /Script/Engine.KismetMaterialLibrary))
  (Variables|Default|SetPlayer _returnvalue_2)
  (bind _returnvalue_3 (Rendering|Material|CreateDynamicMaterialInstance 0 "None" :!class /Script/Engine.KismetMaterialLibrary))
  (Variables|Default|SetLocation _returnvalue_3))

(fn DrawRadar
  (params (Radar%20Size :type Vector%202D%20Structure) (X%20Position :type Float%20%28single-precision%29) (Y%20Position :type Float%20%28single-precision%29))
  (bind (_x _y) (Math|Vector2D|BreakVector2D Radar%20Size))
  (Variables|Default|SetStart%20X X%20Position)
  (Variables|Default|SetStart%20Y Y%20Position)
  (bind _outactors (Actor|GetAllActorsOfClass "/Game/ProjectBase/Blueprint/GeoCache_Blueprint.GeoCache_Blueprint_C"))
  (for _array_element _outactors
    (bind _actor (Utilities|IsinRange _array_element)
      (:In%20Range
        (bind (_radar_position _radar_center) (CallFunction|GetRadarPosition _actor Radar%20Size))
        (bind _radar_rotation (CallFunction|GetRadarRotation))
        (bind _new_point (CallFunction|RotatePoint _radar_position _radar_center _radar_rotation))
        (bind (_new_x _new_y) (CallFunction|GetTempOffset (.X (Math|Vector2D|BreakVector2D _new_point)) (.Y (Math|Vector2D|BreakVector2D _new_point))))
        ;[1 1 1] Draw Location
        (CallFunction|DrawSmartTexture _new_x _new_y 5.0 5.0 "(X=1920.000000,Y=1080.000000)" (Variables|Default|GetLocation)))))
  ;[1 1 1] Draw Player
  (bind (_new_x_2 _new_y_2) (CallFunction|GetTempOffset (/ _x 2.0) (/ _y 2.0)))
  (CallFunction|DrawSmartTexture _new_x_2 _new_y_2 25.0 25.0 "(X=1920.000000,Y=1080.000000)" (Variables|Default|GetPlayer))
  ;[1 1 1] Draw Radar
  (bind (_new_x_3 _new_y_3) (CallFunction|GetTempOffset 0.0 0.0))
  (CallFunction|DrawSmartTexture _new_x_3 _new_y_3 _x _y "(X=1920.000000,Y=1080.000000)" (Variables|Default|GetRadarBG)))

(fn GetRadarPosition
  (params (Detected%20Actor :type Actor%20Object%20Reference) (Radar%20Size :type Vector%202D%20Structure))
  (bind _returnvalue (Game|Player|GetPlayerPawn 0))
  (bind _returnvalue_2 (Transformation|GetActorLocation Detected%20Actor))
  (bind (_x _y) (Math|Vector2D|BreakVector2D Radar%20Size))
  (bind _target_radar_radius (Variables|Default|GetTarget%20Radar%20Radius))
  (bind _returnvalue_3 (Transformation|GetActorLocation _returnvalue))
  (bind _returnvalue_4 (/ _y 2.0))
  (bind _returnvalue_5 (/ _x 2.0))
  (bind _returnvalue_6 (- _returnvalue_3 _returnvalue_2))
  (bind (_x_2 _y_2) (Math|Vector|BreakVector _returnvalue_6))
  (return (Math|Vector2D|MakeVector2D (+ (* _returnvalue_5 (/ _x_2 _target_radar_radius)) _returnvalue_5) (+ (* (/ _y_2 _target_radar_radius) _returnvalue_4) _returnvalue_4)) (Math|Vector2D|MakeVector2D _returnvalue_5 _returnvalue_4)))

(fn GetTempOffset
  (params (X%20Offset :type Float%20%28single-precision%29) (Y%20Offset :type Float%20%28single-precision%29))
  (return X%20Offset Y%20Offset))

(fn DrawSmartTexture
  (params (X%20Pos :type Float%20%28single-precision%29) (Y%20Pos :type Float%20%28single-precision%29) (Width :type Float%20%28single-precision%29) (Height :type Float%20%28single-precision%29) (Ideal%20Screen%20Size :type Vector%202D%20Structure) (Material :type Material%20Instance%20Object%20Reference))
  (bind (_xpos _ypos _scale_width _scale_height) (CallFunction|GetAdjustedScreenPosandSize X%20Pos Y%20Pos Width Height Ideal%20Screen%20Size)))

(fn GetRadarRotation
  (return (* (/ (Math|Float|MultiplybyPi (Math|Float|%(Float) (+ (.Yaw (Math|Rotator|BreakRotator (Pawn|GetControlRotation (Game|GetPlayerController 0) :!class /Script/Engine.Controller))) 2.7e+02) 3.6e+02)) 1.8e+02) -1.0)))

(fn RotatePoint
  (params (Point%20to%20Rotate :type Vector%202D%20Structure) (Center%20Point :type Vector%202D%20Structure) (Angle%20in%20Rad :type Float%20%28single-precision%29))
  (bind (_x _y) (Math|Vector2D|BreakVector2D Point%20to%20Rotate))
  (bind (_x_2 _y_2) (Math|Vector2D|BreakVector2D Center%20Point))
  (return (Math|Vector2D|MakeVector2D (+ (- (* (Math|Trig|Cos(Radians) Angle%20in%20Rad) (- _x _x_2)) (* (Math|Trig|Sin(Radians) Angle%20in%20Rad) (- _y _y_2))) _x_2) (+ _y_2 (+ (* (Math|Trig|Sin(Radians) Angle%20in%20Rad) (- _x _x_2)) (* (Math|Trig|Cos(Radians) Angle%20in%20Rad) (- _y _y_2)))))))

(fn GetAdjustedScreenPosandSize
  (params (XPosIn :type Float%20%28single-precision%29) (YPosIn :type Float%20%28single-precision%29) (Width :type Float%20%28single-precision%29) (Height :type Float%20%28single-precision%29) (Ideal%20Screen%20Size :type Vector%202D%20Structure))
  (bind (_x _y) (Math|Vector2D|BreakVector2D Ideal%20Screen%20Size))
  (bind _screen_dimensions (Variables|Default|GetScreen%20Dimensions))
  (bind (_x_2 _y_2) (Math|Vector2D|BreakVector2D _screen_dimensions))
  (bind _returnvalue (/ _y_2 _y))
  (bind _returnvalue_2 (/ _x_2 _x))
  (return (* XPosIn _returnvalue_2) (* YPosIn _returnvalue) (* Width _returnvalue_2) (* Height _returnvalue) _returnvalue_2 _returnvalue))